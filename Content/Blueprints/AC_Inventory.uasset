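; Inventory component that holds an Items array of SItem structs and provides events to add and remove them.
; AddItem uses CustomFindItem to match by Name and merge stacks, adding Item.Quantity rather than its Quantity input, then prints the array length.
; RemoveItem uses a whole-struct Find, deleting the entry when nothing remains.
; Otherwise it inserts a reduced-quantity copy at that index instead of replacing the original.
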(event `AddItem`
  (params (Item :type "/Game/Structures/S_Item Structure") (Quantity :type Integer :default 1))
  (bind (_name _description _image _asset _quantity) (break `/Game/Structures/S_Item` Item))
  (bind _items (`self.items`))
  (bind _returnvalue (`KismetStringLibrary.Conv_IntToString` (`KismetArrayLibrary.Array_Length` (`self.items`))))
  (bind (_array_index _quantity_2 _found) (`self.CustomFindItem` _items Item))
  (if _found
    (`KismetArrayLibrary.Array_Set` _items _array_index (make `/Game/Structures/S_Item` _name _description _image _asset (+ _quantity_2 _quantity)))
    (`KismetSystemLibrary.PrintString` _returnvalue)
    (else
      (`KismetArrayLibrary.Array_Add` _items Item)
      (`KismetSystemLibrary.PrintString` _returnvalue))))

(event `RemoveItem`
  (params (Item :type "/Game/Structures/S_Item Structure") (Quantity :type Integer :default 1))
  (bind _items (`self.items`))
  (bind _returnvalue (`KismetArrayLibrary.Array_Find` _items Item))
  (bind (_name _description _image _asset _quantity) (break `/Game/Structures/S_Item` (`|GetArrayItem` _items _returnvalue)))
  (bind _returnvalue_2 (- _quantity Quantity))
  (if (> _returnvalue_2 0)
    (`KismetArrayLibrary.Array_Insert` _items (make `/Game/Structures/S_Item` _name _description _image _asset _returnvalue_2) _returnvalue)
    (else
      (`KismetArrayLibrary.Array_Remove` _items _returnvalue))))

(fn `CustomFindItem`
  (params (Array :type "Array of /Game/Structures/S_Item Structure") (ItemToFind :type "/Game/Structures/S_Item Structure"))
  (returns (`Array Index` :type Integer) (Quantity :type Integer) (Found :type Boolean))
  (locals (foundIndex :type Integer) (foundQuantity :type Integer) (`wasFound?` :type Boolean))
  (for (_array_element _array_index) Array
    (bind (_name _description _image _asset _quantity) (break `/Game/Structures/S_Item` _array_element))
    (if (`KismetTextLibrary.EqualEqual_TextText` _name (`.Name_8_8977D90F4AE70E9417DA378CA0EF663E` (break `/Game/Structures/S_Item` ItemToFind)))
      (set `local.foundIndex` _array_index)
      (set `local.foundQuantity` _quantity)
      (set `local.wasFound?` true)
      (break)))
  (return (`local.foundIndex`) (`local.foundQuantity`) (`local.wasFound?`)))