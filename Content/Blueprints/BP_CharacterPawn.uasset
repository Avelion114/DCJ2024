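; Player pawn with grid-based movement and rotation, melee combos and arrow shots, driven by Enhanced Input.
; Melee picks a random combo and finds montages by combo and attack number; presses during an attack are buffered for AttackCombo to continue the chain.
; BeginPlay creates the combat HUD and main menu, which a FlipFlop toggles along with game pause.
; The pick-item input adds a hardcoded Dagger from DT_Items to the inventory component.
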(event `self.ReceiveBeginPlay`
  (`EnhancedInputSubsystemInterface.AddMappingContext` (pcsubsystem `EnhancedInputLocalPlayerSubsystem` (`GameplayStatics.GetPlayerController` 0)) "/Game/Input/IMC_Player.IMC_Player" 0 (struct))
  (`|ExecutionSequence`
    (:`then_0`
      (bind _returnvalue (`|CreateWidget` "/Game/Ui/MainMenu/WB_MainMenu.WB_MainMenu_C" (`GameplayStatics.GetPlayerController` 0)))
      (bind _output_get (set `self.MainMenuRef` _returnvalue))
      (`UserWidget.AddToViewport` _output_get 0))
    (:`then_1`
      (bind _returnvalue_2 (`|CreateWidget` "/Game/Ui/Player/HUD/WB_PlayerCombat_HUD.WB_PlayerCombat_HUD_C" (`GameplayStatics.GetPlayerController` 0)))
      (`UserWidget.AddToViewport` _returnvalue_2 0))))

(event `EnhancedInput|/Game/Input/Actions/IA_Movement`
  (params (ActionValue :type "Vector2D Structure") (ElapsedSeconds :type "Float (double-precision)") (TriggeredSeconds :type "Float (double-precision)") (InputAction :type "InputAction Object Reference" :default "/Game/Input/Actions/IA_Movement.IA_Movement"))
  (:`Triggered`
    (`GridPawnMovementComponent.Move` (`self.GridPawnMovement`) (`KismetMathLibrary.Conv_Vector2DToIntPoint` ActionValue))))

(event `EnhancedInput|/Game/Input/Actions/IA_Rotate`
  (params (ActionValue :type "Float (double-precision)") (ElapsedSeconds :type "Float (double-precision)") (TriggeredSeconds :type "Float (double-precision)") (InputAction :type "InputAction Object Reference" :default "/Game/Input/Actions/IA_Rotate.IA_Rotate"))
  (:`Triggered`
    (`GridPawnMovementComponent.Rotate` (`self.GridPawnMovement`) ActionValue)))

(event `EnhancedInput|/Game/Input/Actions/IA_Menu`
  (params (ActionValue :type Boolean) (ElapsedSeconds :type "Float (double-precision)") (TriggeredSeconds :type "Float (double-precision)") (InputAction :type "InputAction Object Reference" :default "/Game/Input/Actions/IA_Menu.IA_Menu"))
  (bind _mainmenuref (`self.MainMenuRef`))
  (:`Triggered`
    (`/Engine/EditorBlueprintResources/StandardMacros.FlipFlop` :!label _label
      (:`A`
        (`Widget.SetVisibility` _mainmenuref "Visible")
        (`GameplayStatics.SetGamePaused` true))
      (:`B`
        (`Widget.SetVisibility` _mainmenuref "Hidden")
        (`GameplayStatics.SetGamePaused` false)))))

(event `CloseMenu`
  (goto _label))

(event `EnhancedInput|/Game/Input/Actions/IA_MeeleAttack`
  (params (ActionValue :type Boolean) (ElapsedSeconds :type "Float (double-precision)") (TriggeredSeconds :type "Float (double-precision)") (InputAction :type "InputAction Object Reference" :default "/Game/Input/Actions/IA_MeeleAttack.IA_MeeleAttack"))
  (:`Triggered`
    (`self.Attack`)))

(event `EnhancedInput|/Game/Input/Actions/IA_RangedAttack`
  (params (ActionValue :type Boolean) (ElapsedSeconds :type "Float (double-precision)") (TriggeredSeconds :type "Float (double-precision)") (InputAction :type "InputAction Object Reference" :default "/Game/Input/Actions/IA_RangedAttack.IA_RangedAttack"))
  (:`Triggered`
    (`|SpawnActorFromClass` "/Game/Blueprints/BP_Arrow.BP_Arrow_C" (`SceneComponent.K2_GetComponentToWorld` (`self.ArrowDirection`)) "Undefined" "MultiplyWithRoot" null null)))

(event `Attack`
  (if (`self.CanAttack?`)
    (if (`self.Attacking?`)
      (set `self.SaveAtack` true)
      (else
        (set `self.Attacking?` true)
        (set `self.Combo Number` (`KismetMathLibrary.RandomIntegerInRange` 1 2))
        (switch `int` (`self.Attack Counter`) :!label _label_2
          (:`0`
            (bind _anim_montage (`self.Find Attack Montage` (`self.Combo Number`) 1))
            (`self.PlayMontage` _anim_montage))
          (:`1`
            (bind _anim_montage_2 (`self.Find Attack Montage` (`self.Combo Number`) 2))
            (`self.PlayMontage` _anim_montage_2))
          (:`2`
            (bind _anim_montage_3 (`self.Find Attack Montage` (`self.Combo Number`) 3))
            (`self.PlayMontage` _anim_montage_3)))))))

(event `Attack Combo`
  (if (`self.SaveAtack`)
    (set `self.SaveAtack` false)
    (goto _label_2)
    (else
      (`self.Combo End`))))

(event `Combo End`
  (set `self.Attack Counter` 0)
  (set `self.Attacking?` false))

(event `EnhancedInput|/Game/Input/Actions/IA_PickItem`
  (params (ActionValue :type Boolean) (ElapsedSeconds :type "Float (double-precision)") (TriggeredSeconds :type "Float (double-precision)") (InputAction :type "InputAction Object Reference" :default "/Game/Input/Actions/IA_PickItem.IA_PickItem"))
  (:`Triggered`
    (bind _returnvalue (`|GetDataTableRow` "/Game/Structures/DT_Items.DT_Items" "Dagger")
      (:`then`
        (`/Game/Blueprints/AC_Inventory.AddItem` (`self.AC_Inventory`) _returnvalue 1)))))

(fn `Find Attack Montage`
  (params (ComboNumber :type Integer) (AttackNumber :type Integer))
  (returns (`Anim montage` :type "AnimMontage Object Reference"))
  (bind _keys (`BlueprintMapLibrary.Map_Keys` (`self.Attack Montages`)))
  (for _array_element _keys
    (bind (_combonumber _attacknumber) (break `/Game/Structures/S_FightMontageInfo` (`BlueprintMapLibrary.Map_Find` (`self.Attack Montages`) _array_element)))
    (if (== _combonumber ComboNumber)
      (if (== _attacknumber AttackNumber)
        (return _array_element)))))

(fn `UserConstructionScript`)