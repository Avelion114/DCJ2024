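; Grid spawner that builds a dungeon crawler level from layer 0 of a tile map when play begins.
; Reset clears spawned actors and all dungeon pieces, then spawns walls or floors by tile index at GridSize spacing.
; Floor cells are recorded by coordinate, with one tile type tagged "Start".
; Setup copies them into the game instance's GridSpaces, and the startup delegate fires a tick later.
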(event `self.ReceiveBeginPlay`
  (`self.Setup`)
  (`KismetSystemLibrary.DelayUntilNextTick`)
  (`DungeonCrawlerGameInstance.StartupDelegate` (cast `DungeonCrawlerGameInstance` (`GameplayStatics.GetGameInstance`) :!pure true)))

(event `Reset`
  (`self.ClearMap`)
  (`self.GetSpawnData`))

(event `GetSpawnData`
  (bind _rendercomponent (`PaperTileMapActor.RenderComponent` (`self.TileMap`)))
  (bind _tilemap (`PaperTileMapComponent.TileMap` _rendercomponent))
  (for _index (range (`PaperTileMap.MapHeight` _tilemap))
    (for _index_2 (range (`PaperTileMap.MapWidth` _tilemap))
      (bind (_tileindex _tileset _bfliph _bflipv _bflipd) (`TileMapBlueprintLibrary.BreakTile` (`PaperTileMapComponent.GetTile` _rendercomponent _index_2 _index 0)))
      (`self.SpawnWorld` (make `IntPoint` _index_2 _index) _tileindex _bflipd))))

(event `SpawnWorld`
  (params (Coordinate1 :type "IntPoint Structure") (Index1 :type Integer) (Rotated1 :type Boolean))
  (bind (_x _y) (break `IntPoint` Coordinate1))
  (bind _gridsize (`self.GridSize`))
  (bind _returnvalue (+ (`self.K2_GetActorLocation`) (`KismetMathLibrary.MakeVector` (* _x _gridsize) (* _y _gridsize))))
  (switch `int` Index1
    (:`1`
      (bind _returnvalue_2 (`|SpawnActorFromClass` "/Game/Blueprints/TileMapStuff/Actors/BP_Wall.BP_Wall_C" (`KismetMathLibrary.MakeTransform` _returnvalue (struct)) "Undefined" "MultiplyWithRoot" null null))
      (`KismetArrayLibrary.Array_Add` (`self.Actors`) _returnvalue_2))
    (:`2`
      (bind _returnvalue_3 (`|SpawnActorFromClass` "/Game/Blueprints/TileMapStuff/Actors/BP_Floor.BP_Floor_C" (`KismetMathLibrary.MakeTransform` _returnvalue) "Undefined" "MultiplyWithRoot" null null :!label _label))
      (`KismetArrayLibrary.Array_Add` (`self.Actors`) _returnvalue_3)
      (`BlueprintMapLibrary.Map_Add` (`self.FloorData`) Coordinate1 (select `bool` (== Index1 3) :`false` (make `GridSpaceData` _returnvalue) :`true` (make `GridSpaceData` _returnvalue (`|MakeArray` "Start" :!type "Name")))))
    (:`3`
      (goto _label))))

(event `ClearMap`
  (`BlueprintMapLibrary.Map_Clear` (`self.FloorData`))
  (for _array_element (`self.Actors`)
    (`self.K2_DestroyActor` _array_element))
  (bind _outactors (`GameplayStatics.GetAllActorsOfClass` "/Game/Blueprints/TileMapStuff/Actors/BP_DungeonPiece.BP_DungeonPiece_C"))
  (for _array_element_2 _outactors
    (`self.K2_DestroyActor` _array_element_2)))

(fn `Setup`
  (bind _floordata (`self.FloorData`))
  (`self.Reset`)
  (bind _keys (`BlueprintMapLibrary.Map_Keys` _floordata))
  (for _array_element _keys
    (`BlueprintMapLibrary.Map_Add` (`DungeonCrawlerGameInstance.GridSpaces` (cast `DungeonCrawlerGameInstance` (`GameplayStatics.GetGameInstance`) :!pure true)) _array_element (`BlueprintMapLibrary.Map_Find` _floordata _array_element))))

(fn `UserConstructionScript`)