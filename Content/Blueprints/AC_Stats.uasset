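; AC_Stats is a component, by its prefix, that tracks player health and hunger.
; Both stats start at their maximums, and hunger drops by a fixed amount every tick, unscaled by delta time and without a floor.
; Damage calls PlayerDefeated when health reaches zero or below, otherwise plays a 2D hurt sound.
; Healing adds health, capped at the maximum.
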(event `self.ReceiveBeginPlay`
  (set `self.CurrentHunger` (`self.MaxHunger`))
  (set `self.CurrentHealth` (`self.MaxHealth`)))

(event `self.ReceiveTick`
  (params (DeltaSeconds :type "Float (single-precision)"))
  (set `self.CurrentHunger` (- (`self.CurrentHunger`) 0.01)))

(event `DamagePlayer`
  (params (DamageAmount :type "Float (double-precision)"))
  (bind _output_get (set `self.CurrentHealth` (- (`self.CurrentHealth`) DamageAmount)))
  (if (<= _output_get 0.0)
    (`self.PlayerDefeated`)
    (else
      (`GameplayStatics.PlaySound2D` "/Game/Audio/AxSFX/Player/Sfx_Plyr_TkDamage.Sfx_Plyr_TkDamage" 1.0 1.0 0.0 null null))))

(event `HealPlayer`
  (params (HealAmount :type "Float (double-precision)"))
  (bind _output_get (set `self.CurrentHealth` (+ (`self.CurrentHealth`) HealAmount)))
  (if (>= _output_get (`self.MaxHealth`))
    (set `self.CurrentHealth` (`self.MaxHealth`))))