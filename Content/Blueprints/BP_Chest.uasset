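; BP_Chest is an interactable dungeon chest that randomly either bites the player or plays a give-item animation.
; BeginPlay rolls WillBite and passes it to the chest sound as a seed.
; Box overlap shows the prompt widget and enables IA_PickItem, which plays the matching montage, damaging the player on a bite.
; Both outcomes then loop a lick animation, notify DungeonCrawlerGameMode via ChestFound and destroy the chest after delays.
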(event `self.ReceiveBeginPlay`
  (bind _output_get (set `self.bWillBite` (`KismetMathLibrary.RandomBool`)))
  (`AudioParameterControllerInterface.SetIntParameter` (`self.SFX_Chest`) "Seed" (`KismetMathLibrary.Conv_BoolToInt` _output_get))
  (bind _asbp_character_pawn (cast `/Game/Blueprints/BP_CharacterPawn` (`GameplayStatics.GetPlayerPawn` 0)))
  (set `self.As BP Character Pawn` _asbp_character_pawn))

(event `self.Box.OnComponentBeginOverlap`
  (params (OverlappedComponent :type "PrimitiveComponent Object Reference") (OtherActor :type "Actor Object Reference") (OtherComp :type "PrimitiveComponent Object Reference") (OtherBodyIndex :type Integer) (bFromSweep :type Boolean) (SweepResult :type "HitResult Structure (by ref)"))
  ;[0.4742 0.3646 1] Player Enter/Exit
  (if (== OtherActor (`GameplayStatics.GetPlayerPawn` 0))
    (`SceneComponent.SetHiddenInGame` (`self.Widget`) false false)
    (set `self.bCanInteract` true)))

(event `self.Box.OnComponentEndOverlap`
  (params (OverlappedComponent :type "PrimitiveComponent Object Reference") (OtherActor :type "Actor Object Reference") (OtherComp :type "PrimitiveComponent Object Reference") (OtherBodyIndex :type Integer))
  ;[0.4742 0.3646 1] Player Enter/Exit
  (if (== (`GameplayStatics.GetPlayerPawn` 0) OtherActor)
    (`SceneComponent.SetHiddenInGame` (`self.Widget`) true false)
    (set `self.bCanInteract` false)))

(event `EnhancedInput|/Game/Input/Actions/IA_PickItem`
  (params (ActionValue :type Boolean) (ElapsedSeconds :type "Float (double-precision)") (TriggeredSeconds :type "Float (double-precision)") (InputAction :type "InputAction Object Reference" :default "/Game/Input/Actions/IA_PickItem.IA_PickItem"))
  (:`Triggered`
    (if (`self.bCanInteract`)
      (set `self.bCanInteract` false)
      (`AudioParameterControllerInterface.SetTriggerParameter` (`self.SFX_Chest`) "PlayInteract")
      (if (`self.bWillBite`)
        (`|PlayMontage` (`self.Chest`) "/Game/ArtContent/Animations/AN_Seq/Chest/AN_Chest_Bite_Montage.AN_Chest_Bite_Montage"
          (:`then`
            (`/Game/Blueprints/AC_Stats.DamagePlayer` (`/Game/Blueprints/BP_CharacterPawn.AC_Stats` (`self.As BP Character Pawn`)) 1.0))
          (:`OnCompleted`
            _))
        (else
          (`|PlayMontage` (`self.Chest`) "/Game/ArtContent/Animations/AN_Seq/Chest/AN_Chest_GiveItem_Montage.AN_Chest_GiveItem_Montage"
            (:`OnCompleted`
              _))))
      (`KismetSystemLibrary.Delay` 3.0)
      (`SkeletalMeshComponent.PlayAnimation` (`self.Chest`) "/Game/ArtContent/Animations/AN_Seq/Chest/AN_Chest_Lick.AN_Chest_Lick" true)
      (`/Game/GameData/DungeonCrawlerGameMode.ChestFound` (cast `/Game/GameData/DungeonCrawlerGameMode` (`GameplayStatics.GetGameMode`) :!pure true))
      (`KismetSystemLibrary.Delay` 5.0)
      (`self.K2_DestroyActor`))))

(event `BitePlayer`
  (`|PlayMontage` (`self.Chest`) "/Game/ArtContent/Animations/AN_Seq/Chest/AN_Chest_Bite_Montage.AN_Chest_Bite_Montage"
    (:`then`
      (`|PlayMontage` null "/Game/ArtContent/Animations/AN_Seq/Arms/AN_Looting_Bit_Anim_Montage.AN_Looting_Bit_Anim_Montage"))))

(event `RewardPlayer`
  (`|PlayMontage` (`self.Chest`) "/Game/ArtContent/Animations/AN_Seq/Chest/AN_Chest_GiveItem_Montage.AN_Chest_GiveItem_Montage"
    (:`then`
      (`|PlayMontage` null "/Game/ArtContent/Animations/AN_Seq/Arms/AN_Looting_Safe_Anim_Montage.AN_Looting_Safe_Anim_Montage"))))

(fn `UserConstructionScript`)