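; Enemy pawn for a grid-based dungeon crawler that chases the player from cell to cell.
; On BeginPlay, marked as testing only, it teleports to a random GridSpaces cell and, after short delays, requests a path to the player from GridAIController.
; It reverses that path and walks it through GridPawnMovement, requesting a new one when the steps run out.
; Debug path drawing and random-target logic are disconnected.
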(event `self.ReceiveBeginPlay`
  (bind _gridspaces (`DungeonCrawlerGameInstance.GridSpaces` (cast `DungeonCrawlerGameInstance` (`GameplayStatics.GetGameInstance`) :!pure true)))
  ;[1 0.6754 0] Testing Only
  (`KismetSystemLibrary.Delay` 0.5)
  (bind _keys (`BlueprintMapLibrary.Map_Keys` _gridspaces))
  (bind _output_get (set `self.Location` (`|GetArrayItem` _keys (`KismetMathLibrary.RandomInteger` (`KismetArrayLibrary.Array_Length` _keys)))))
  (`GridPawnMovementComponent.SetCoordinates` (`self.GridPawnMovement`) _output_get)
  (`self.K2_SetActorLocation` (break `GridSpaceData` (`BlueprintMapLibrary.Map_Find` _gridspaces _output_get)))
  (add `GridPawnMovementComponent.MoveComplete` (`self.GridPawnMovement`) (`|CreateDelegate` :!event `FollowPath`))
  (`KismetSystemLibrary.Delay` 1.0)
  (`self.GetPathToPlayer`))

(event `GetPathToPlayer`
  ;[1 0.6754 0] Testing Only
  (bind _returnvalue (`GridAIController.GetPathToLocation` (cast `GridAIController` (`self.GetController`) :!pure true) (`GridPawnMovementComponent.GetCoordinates` (`self.GridPawnMovement`)) (`GridPawnMovementComponent.GetCoordinates` (`/Game/Blueprints/BP_CharacterPawn.GridPawnMovement` (cast `/Game/Blueprints/BP_CharacterPawn` (`GameplayStatics.GetPlayerPawn` 0) :!pure true)))))
  (set `self.Path` _returnvalue)
  (`KismetArrayLibrary.Array_Reverse` (`self.Path`))
  (`self.FollowPath`))

(event `self.ReceiveTick`
  (params (DeltaSeconds :type "Float (single-precision)"))
  ;[1 0.6754 0] Testing Only
)

(event `FollowPath`
  (bind _pathindex (`self.PathIndex`))
  (bind _path (`self.Path`))
  (`/Engine/EditorBlueprintResources/StandardMacros.IncrementInt` (`self.PathIndex`)
    (:`  `
      (if (`KismetArrayLibrary.Array_IsValidIndex` _path _pathindex)
        (`GridPawnMovementComponent.Move` (`self.GridPawnMovement`) (- (`|GetArrayItem` _path _pathindex) (`GridPawnMovementComponent.GetCoordinates` (`self.GridPawnMovement`))))
        (else
          (set `self.PathIndex` -1)
          (`self.GetPathToPlayer`))))))

(fn `UserConstructionScript`)