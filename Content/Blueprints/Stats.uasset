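; Stats Blueprint that tracks the player's hunger and health, both set to their maximums on BeginPlay.
; Hunger drains by a fixed amount every Tick, without delta-time scaling, and TakeDamage subtracts incoming damage from health.
; Either value reaching zero or below leads to a shared "Player Defeated" print, which repeats every Tick while hunger stays depleted.
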(event `self.ReceiveBeginPlay`
  (set `self.CurrentHunger` (`self.MaxHunger`))
  (set `self.CurrentHealth` (`self.MaxHealth`)))

(event `self.ReceiveTick`
  (params (DeltaSeconds :type "Float (single-precision)"))
  (bind _output_get (set `self.CurrentHunger` (- (`self.CurrentHunger`) 0.01)))
  (if (<= _output_get 0.0)
    (`KismetSystemLibrary.PrintString` "Player Defeated" :!label _label)))

(event `TakeDamage`
  (params (DamageAmount :type "Float (double-precision)"))
  (bind _output_get (set `self.CurrentHealth` (- (`self.CurrentHealth`) DamageAmount)))
  (if (<= _output_get 0.0)
    (goto _label)))