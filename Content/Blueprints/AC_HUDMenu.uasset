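; AC_HUDMenu is a component that swaps between a paused main menu and the player combat HUD.
; BeginPlay and the menu input, gated by a DoOnce, share one path that creates WB_MainMenu if its reference is invalid, shows the cursor and pauses.
; The menu's CloseMenu dispatcher unpauses, replaces it with a new WB_PlayerCombat_HUD and resets the DoOnce.
; An older FlipFlop visibility toggle remains unconnected.
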(event `self.ReceiveBeginPlay`
  (bind _returnvalue (`GameplayStatics.GetPlayerController` 0))
  (`self.MainMenuRef` :!label _label
    (:`then`)
    (:`else`
      (bind _playerhud (`self.PlayerHUD`)
        (:`then`
          (`Widget.RemoveFromParent` _playerhud))
        (:`else`
          _))
      (bind _returnvalue_2 (`|CreateWidget` "/Game/Ui/MainMenu/WB_MainMenu.WB_MainMenu_C" (`GameplayStatics.GetPlayerController` 0)))
      (bind _output_get (set `self.MainMenuRef` _returnvalue_2))
      (`UserWidget.AddToViewport` _output_get 0)
      (`WidgetBlueprintLibrary.SetInputMode_GameAndUIEx` _returnvalue (`self.MainMenuRef`) "DoNotLock" false)
      (set `PlayerController.bShowMouseCursor` true _returnvalue)
      (`GameplayStatics.SetGamePaused` true)
      (add `/Game/Ui/MainMenu/WB_MainMenu.CloseMenu` (`self.MainMenuRef`) (delegate `CloseMenu_Event`)))))

(event `IA_MenuButton`
  (`/Engine/EditorBlueprintResources/StandardMacros.DoOnce` false :!label _label_2
    (:`Completed`
      (goto _label))))

(event `CloseMenu_Event`
  (`GameplayStatics.SetGamePaused` false)
  (`self.AddPlayerHUD`)
  (`self.ResetMenuDoOnce`))

(event `ResetMenuDoOnce`
  (goto _label_2 :!via `Reset`))

(event `AddPlayerHUD`
  (bind _mainmenuref (`self.MainMenuRef`)
    (:`then`
      (`Widget.RemoveFromParent` _mainmenuref)
      (bind _returnvalue (`|CreateWidget` "/Game/Ui/Player/HUD/WB_PlayerCombat_HUD.WB_PlayerCombat_HUD_C" (`GameplayStatics.GetPlayerController` 0)))
      (bind _output_get (set `self.PlayerHUD` _returnvalue))
      (`UserWidget.AddToViewport` _output_get 0)
      (`WidgetBlueprintLibrary.SetInputMode_GameAndUIEx` (`GameplayStatics.GetPlayerController` 0) (`self.PlayerHUD`) "DoNotLock" false))
    (:`else`)))